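; BP_BananaBullet is a projectile that damages monkey enemies on impact.
; It captures its forward vector at BeginPlay and moves along it each Tick with a swept world offset.
; The first sphere hit clears CanHit, so the next Tick destroys the bullet.
; A cast chain over four monkey types subtracts Health directly and sets State from whether Health is depleted, with debug prints.
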(event OnComponentHit(Sphere1)
  (params (HitComponent :type Primitive%20Component%20Object%20Reference) (OtherActor :type Actor%20Object%20Reference) (OtherComp :type Primitive%20Component%20Object%20Reference) (NormalImpulse :type Vector :default "0, 0, 0") (Hit :type Hit%20Result%20Structure%20%28by%20ref%29))
  (if (Variables|Default|GetCanHit)
    (Variables|Default|SetCanHit false)
    ;[0.15 0.15 0.15 0.5] debugging
    (Development|PrintString "HIT")
    ;[0.15 0.15 0.15 0.5] Monkey "rage decreasing" logic (damage :|)
    (bind _asbp_beefy_monkey (Utilities|Casting|CastToBP_BeefyMonkey OtherActor)
      (:then
        (bind _output_get (Variables|/Game/Blueprints/BP_BeefyMonkey.BP_BeefyMonkey_C|SetHealth _asbp_beefy_monkey (- (Variables|/Game/Blueprints/BP_BeefyMonkey.BP_BeefyMonkey_C|GetHealth _asbp_beefy_monkey) 1e+01)))
        (Variables|/Game/Blueprints/BP_BeefyMonkey.BP_BeefyMonkey_C|SetState _asbp_beefy_monkey (<= _output_get 0.0)))
      (:CastFailed
        (bind _asbp_quick_monkey (Utilities|Casting|CastToBP_QuickMonkey OtherActor)
          (:then
            (bind _output_get_2 (Variables|/Game/Blueprints/BP_QuickMonkey.BP_QuickMonkey_C|SetHealth _asbp_quick_monkey (- (Variables|/Game/Blueprints/BP_QuickMonkey.BP_QuickMonkey_C|GetHealth _asbp_quick_monkey) 1e+01)))
            (Variables|/Game/Blueprints/BP_QuickMonkey.BP_QuickMonkey_C|SetState _asbp_quick_monkey (<= _output_get_2 0.0)))
          (:CastFailed
            (bind _asbp_sneaky_monkey (Utilities|Casting|CastToBP_SneakyMonkey OtherActor)
              (:then
                (bind _output_get_3 (Variables|/Game/Blueprints/BP_SneakyMonkey.BP_SneakyMonkey_C|SetHealth _asbp_sneaky_monkey (- (Variables|/Game/Blueprints/BP_SneakyMonkey.BP_SneakyMonkey_C|GetHealth _asbp_sneaky_monkey) 1e+01)))
                (Variables|/Game/Blueprints/BP_SneakyMonkey.BP_SneakyMonkey_C|SetState _asbp_sneaky_monkey (<= _output_get_3 0.0)))
              (:CastFailed
                (bind _asbp_common_monkey (Utilities|Casting|CastToBP_CommonMonkey OtherActor)
                  (:then
                    (bind _output_get_4 (Variables|/Game/Blueprints/BP_CommonMonkey.BP_CommonMonkey_C|SetHealth _asbp_common_monkey (- (Variables|/Game/Blueprints/BP_CommonMonkey.BP_CommonMonkey_C|GetHealth _asbp_common_monkey) 1e+01)))
                    (Variables|/Game/Blueprints/BP_CommonMonkey.BP_CommonMonkey_C|SetState _asbp_common_monkey (<= _output_get_4 0.0)))
                  (:CastFailed
                    ;[0.15 0.15 0.15 0.5] debugging
                    (Development|PrintString (Utilities|GetDisplayName OtherActor))))))))))))

(event EventBeginPlay
  (Variables|Default|SetDirection (Transformation|GetActorForwardVector)))

(event Collision|EventActorBeginOverlap
  (params (OtherActor :type Actor%20Object%20Reference)))

(event EventTick
  (params (DeltaSeconds :type Float%20%28single-precision%29))
  ;[0.15 0.15 0.15 0.5] Keep the projectile moving in a line
  (Transformation|AddActorWorldOffset (* (* (Variables|Default|GetDirection) DeltaSeconds) 1e+03) true)
  (if (not (Variables|Default|GetCanHit))
    (Actor|DestroyActor)))

(fn ConstructionScript)