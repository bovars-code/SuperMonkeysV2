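; Waypoint marker actor that hovers high above a referenced component and fades out as the player approaches it.
; BeginPlay creates a dynamic material on its sphere and applies color and emissivity.
; Each Tick, while the referenced component is not below zero height, the actor copies its X and Y at a fixed altitude.
; The player's horizontal distance to the sphere then drives opacity, dropping to invisible at close range.
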(event EventBeginPlay
  (bind _returnvalue (Rendering|Material|CreateDynamicMaterialInstance (Variables|Default|GetSphere) 0 "/Game/Blueprints/M_Waypoint.M_Waypoint" "None" :!class /Script/Engine.PrimitiveComponent))
  (bind _output_get (Variables|Default|SetMaterialReference _returnvalue))
  (Rendering|Material|SetVectorParameterValue _output_get "Color" (Variables|Default|GetColorStruct) :!class /Script/Engine.MaterialInstanceDynamic)
  (Rendering|Material|SetScalarParameterValue _output_get "Emissivity" (Variables|Default|GetEmissivity) :!class /Script/Engine.MaterialInstanceDynamic))

(event Collision|EventActorBeginOverlap
  (params (OtherActor :type Actor%20Object%20Reference)))

(event EventTick
  (params (DeltaSeconds :type Float%20%28single-precision%29))
  (bind _returnvalue (Game|GetPlayerCharacter 0))
  (bind _materialreference (Variables|Default|GetMaterialReference))
  (bind _referencecomponent (Variables|Default|GetReferenceComponent))
  (bind _sphere (Variables|Default|GetSphere))
  (bind _returnvalue_2 (Transformation|GetWorldLocation _referencecomponent))
  (bind _returnvalue_3 (Transformation|GetWorldLocation _sphere))
  (bind _mesh (Variables|/Script/Engine.Character|GetMesh _returnvalue))
  (bind _returnvalue_4 (Transformation|GetWorldLocation _mesh))
  (bind _returnvalue_5 (Math|Vector|Distance(Vector) (Math|Vector|MakeVector (.x _returnvalue_4) (.y _returnvalue_4) 0.0) (Math|Vector|MakeVector (.x _returnvalue_3) (.y _returnvalue_3) 0.0)))
  (if (not (< (.z _returnvalue_2) 0.0))
    (Transformation|SetActorLocation (Math|Vector|MakeVector (.x _returnvalue_2) (.y _returnvalue_2) 5e+03) false false)
    (if (< _returnvalue_5 2e+03)
      (Rendering|Material|SetScalarParameterValue _materialreference "Opacity" 0.0 :!class /Script/Engine.MaterialInstanceDynamic)
      (else
        (Rendering|Material|SetScalarParameterValue _materialreference "Opacity" (/ _returnvalue_5 3535.0) :!class /Script/Engine.MaterialInstanceDynamic)))))

(fn ConstructionScript)