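; Test planet actor that scatters grass, flowers and trees over a sphere and marks a ship with a waypoint on BeginPlay.
; Golden-angle Fibonacci sphere functions fill ISM and HISM components, adding random jitter and pointing each instance's Z away from the centre.
; It spawns BP_Waypoint at the Ship component.
; Trigger overlap toggles a widget, while IA_Interact opens LVL_SneakyMonkeyMap without checking overlap.
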(event OnComponentBeginOverlap(Trigger)
  (params (OverlappedComponent :type Primitive%20Component%20Object%20Reference) (OtherActor :type Actor%20Object%20Reference) (OtherComp :type Primitive%20Component%20Object%20Reference) (OtherBodyIndex :type Integer) (bFromSweep :type Boolean) (SweepResult :type Hit%20Result%20Structure%20%28by%20ref%29))
  (Rendering|SetVisibility (Variables|Default|GetWidget) true false))

(event OnComponentEndOverlap(Trigger)
  (params (OverlappedComponent :type Primitive%20Component%20Object%20Reference) (OtherActor :type Actor%20Object%20Reference) (OtherComp :type Primitive%20Component%20Object%20Reference) (OtherBodyIndex :type Integer))
  (Rendering|SetVisibility (Variables|Default|GetWidget) false false))

(event Custom|Distribute%20Points
  (CallFunction|FibonacciDistributionISM 5000 (Variables|Default|GetRadius) (Variables|Default|GetISM_Grass) 0.05)
  (CallFunction|FibonacciDistributionHISM 1500 (Variables|Default|GetRadius) (Variables|Default|GetHSIM_Flower) 0.1)
  (CallFunction|FibonacciDistributionHISM 400 (Variables|Default|GetRadius) (Variables|Default|GetHISM_Tree) 0.5))

(event Input|EnhancedActionEvents|EnhancedInputActionIA_Interact
  (params (ActionValue :type Boolean) (ElapsedSeconds :type Float%20%28double-precision%29) (TriggeredSeconds :type Float%20%28double-precision%29) (InputAction :type Input%20Action%20Object%20Reference :default "/Game/Input/Actions/IA_Interact.IA_Interact"))
  ;[0.15 0.15 0.15 0.5] changed to F key in IMC
  (Game|OpenLevel(byName) "LVL_SneakyMonkeyMap"))

(event EventBeginPlay
  (CallFunction|DistributePoints)
  (CallFunction|CreateWaypoint (Variables|Default|GetShip) (Utilities|Struct|MakeLinearColor 1.0 0.0 0.0 1.0) 5.0))

(event Collision|EventActorBeginOverlap
  (params (OtherActor :type Actor%20Object%20Reference)))

(event EventTick
  (params (DeltaSeconds :type Float%20%28single-precision%29)))

(fn ConstructionScript)

(fn FibonacciDistributionHISM
  (params (Density :type Integer) (Radius :type Float%20%28double-precision%29) (Instanced%20Static%20Mesh :type Hierarchical%20Instanced%20Static%20Mesh%20Component%20Object%20Reference) (DisperseLevel :type Float%20%28double-precision%29))
  (for _index (range 0 Density)
    (Components|InstancedStaticMesh|AddInstance Instanced%20Static%20Mesh (Math|Transform|MakeTransform (+ (* (Math|Vector|Normalize (+ (Math|Vector|Normalize (Math|Vector|MakeVector (* (Math|Float|Sqrt (- 1.0 (Math|Float|Square (- 1.0 (* (/ _index (Math|Conversions|ToFloat(Integer) (- Density 1))) 2.0))))) (Math|Trig|Cos(Radians) (* _index (* (- 3.0 (Math|Float|Sqrt 5.0)) (Math|Trig|GetPI))))) (- 1.0 (* (/ _index (Math|Conversions|ToFloat(Integer) (- Density 1))) 2.0)) (* (Math|Float|Sqrt (- 1.0 (Math|Float|Square (- 1.0 (* (/ _index (Math|Conversions|ToFloat(Integer) (- Density 1))) 2.0))))) (Math|Trig|Sin(Radians) (* _index (* (- 3.0 (Math|Float|Sqrt 5.0)) (Math|Trig|GetPI))))))) (* (Math|Random|RandomUnitVector) DisperseLevel))) Radius) (Transformation|GetActorLocation)) (Math|Rotator|MakeRotfromZ (Math|Vector|Normalize (- (+ (* (Math|Vector|Normalize (+ (Math|Vector|Normalize (Math|Vector|MakeVector (* (Math|Float|Sqrt (- 1.0 (Math|Float|Square (- 1.0 (* (/ _index (Math|Conversions|ToFloat(Integer) (- Density 1))) 2.0))))) (Math|Trig|Cos(Radians) (* _index (* (- 3.0 (Math|Float|Sqrt 5.0)) (Math|Trig|GetPI))))) (- 1.0 (* (/ _index (Math|Conversions|ToFloat(Integer) (- Density 1))) 2.0)) (* (Math|Float|Sqrt (- 1.0 (Math|Float|Square (- 1.0 (* (/ _index (Math|Conversions|ToFloat(Integer) (- Density 1))) 2.0))))) (Math|Trig|Sin(Radians) (* _index (* (- 3.0 (Math|Float|Sqrt 5.0)) (Math|Trig|GetPI))))))) (* (Math|Random|RandomUnitVector) DisperseLevel))) Radius) (Transformation|GetActorLocation)) (Transformation|GetActorLocation)))) "1.000000,1.000000,1.000000") true)))

(fn FibonacciDistributionISM
  (params (density :type Integer) (radius :type Float%20%28double-precision%29) (mesh :type Instanced%20Static%20Mesh%20Component%20Object%20Reference) (disperse :type Float%20%28double-precision%29))
  (for _index (range 0 density)
    (Components|InstancedStaticMesh|AddInstance mesh (Math|Transform|MakeTransform (+ (* (Math|Vector|Normalize (+ (Math|Vector|Normalize (Math|Vector|MakeVector (* (Math|Float|Sqrt (- 1.0 (Math|Float|Square (- 1.0 (* (/ _index (Math|Conversions|ToFloat(Integer) (- density 1))) 2.0))))) (Math|Trig|Cos(Radians) (* _index (* (- 3.0 (Math|Float|Sqrt 5.0)) (Math|Trig|GetPI))))) (- 1.0 (* (/ _index (Math|Conversions|ToFloat(Integer) (- density 1))) 2.0)) (* (Math|Float|Sqrt (- 1.0 (Math|Float|Square (- 1.0 (* (/ _index (Math|Conversions|ToFloat(Integer) (- density 1))) 2.0))))) (Math|Trig|Sin(Radians) (* _index (* (- 3.0 (Math|Float|Sqrt 5.0)) (Math|Trig|GetPI))))))) (* (Math|Random|RandomUnitVector) disperse))) radius) (Transformation|GetActorLocation)) (Math|Rotator|MakeRotfromZ (Math|Vector|Normalize (- (+ (* (Math|Vector|Normalize (+ (Math|Vector|Normalize (Math|Vector|MakeVector (* (Math|Float|Sqrt (- 1.0 (Math|Float|Square (- 1.0 (* (/ _index (Math|Conversions|ToFloat(Integer) (- density 1))) 2.0))))) (Math|Trig|Cos(Radians) (* _index (* (- 3.0 (Math|Float|Sqrt 5.0)) (Math|Trig|GetPI))))) (- 1.0 (* (/ _index (Math|Conversions|ToFloat(Integer) (- density 1))) 2.0)) (* (Math|Float|Sqrt (- 1.0 (Math|Float|Square (- 1.0 (* (/ _index (Math|Conversions|ToFloat(Integer) (- density 1))) 2.0))))) (Math|Trig|Sin(Radians) (* _index (* (- 3.0 (Math|Float|Sqrt 5.0)) (Math|Trig|GetPI))))))) (* (Math|Random|RandomUnitVector) disperse))) radius) (Transformation|GetActorLocation)) (Transformation|GetActorLocation)))) "1.000000,1.000000,1.000000") true)))

(fn CreateWaypoint
  (params (ReferenceComponent :type Static%20Mesh%20Component%20Object%20Reference) (Color :type Linear%20Color%20Structure) (Emmissivitty :type Float%20%28double-precision%29))
  (Game|SpawnActorfromClass "/Game/Blueprints/BP_Waypoint.BP_Waypoint_C" (Math|Conversions|ToTransform(Vector) (Transformation|GetWorldLocation (Variables|Default|GetShip))) "Undefined" "MultiplyWithRoot" 0 ReferenceComponent Color Emmissivitty 0))