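; BP_Banana is a banana pickup that gives the first-person character ammo.
; It adds a rotating movement component on BeginPlay and detects collectors through its Sphere1 overlap.
; An overlapping BP_FirstPersonCharacter gains AmmoAmount, the new total is printed, and the banana destroys itself.
; For other actors, the failed cast branch prints the display name of the empty cast result rather than the overlapping actor.
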(event OnComponentBeginOverlap(Sphere1)
  (params (OverlappedComponent :type Primitive%20Component%20Object%20Reference) (OtherActor :type Actor%20Object%20Reference) (OtherComp :type Primitive%20Component%20Object%20Reference) (OtherBodyIndex :type Integer) (bFromSweep :type Boolean) (SweepResult :type Hit%20Result%20Structure%20%28by%20ref%29))
  (bind _asbp_first_person_character (Utilities|Casting|CastToBP_FirstPersonCharacter OtherActor)
    (:then
      (bind _output_get (Variables|/Game/FirstPerson/Blueprints/BP_FirstPersonCharacter.BP_FirstPersonCharacter_C|SetAmmo _asbp_first_person_character (+ (Variables|/Game/FirstPerson/Blueprints/BP_FirstPersonCharacter.BP_FirstPersonCharacter_C|GetAmmo _asbp_first_person_character) (Variables|Default|GetAmmo%20amount))))
      (Development|PrintString (Utilities|String|ToString(Integer) _output_get))
      (Actor|DestroyActor))
    (:CastFailed
      (Development|PrintString (Utilities|GetDisplayName _asbp_first_person_character)))))

(event EventBeginPlay
  (AddComponent|AddRotatingMovementComponent))

(event Collision|EventActorBeginOverlap
  (params (OtherActor :type Actor%20Object%20Reference)))

(event EventTick
  (params (DeltaSeconds :type Float%20%28single-precision%29)))

(fn ConstructionScript)