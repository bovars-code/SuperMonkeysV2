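; BP_BeefyMonkey is an enemy character that chases and lunges at the player, dealing contact damage.
; Looping timers drive an AI move and a jump-then-forward launch, both active only while the player's noticeable range covers it and State is false.
; Capsule overlap subtracts player health and calls Fainted at zero; when State is true, Tick halts movement and flags BDefeat on the player.
; BeginPlay passes itself to the rage meter widget, whose update and camera-facing logic here is unconnected.
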(event OnComponentBeginOverlap(CapsuleComponent)
  (params (OverlappedComponent :type Primitive%20Component%20Object%20Reference) (OtherActor :type Actor%20Object%20Reference) (OtherComp :type Primitive%20Component%20Object%20Reference) (OtherBodyIndex :type Integer) (bFromSweep :type Boolean) (SweepResult :type Hit%20Result%20Structure%20%28by%20ref%29))
  ;[0.15 0.15 0.15 0.5] Remove 10.0 from player's hp, check for faint scenario (Damage)
  (bind _asbp_third_person_character (Utilities|Casting|CastToBP_ThirdPersonCharacter OtherActor))
  (bind _output_get (Variables|/Game/ThirdPerson/Blueprints/BP_ThirdPersonCharacter.BP_ThirdPersonCharacter_C|SetHealth _asbp_third_person_character (- (Variables|/Game/ThirdPerson/Blueprints/BP_ThirdPersonCharacter.BP_ThirdPersonCharacter_C|GetHealth _asbp_third_person_character) 1e+01)))
  (Development|PrintString (Utilities|String|ToString(Float) _output_get))
  (if (<= _output_get 0.0)
    (Default|Fainted _asbp_third_person_character "Beefy Monkey")))

(event Custom|Chase%20Player
  (if (not (Variables|Default|GetState))
    (bind _asbp_third_person_character (Utilities|Casting|CastToBP_ThirdPersonCharacter (Game|GetPlayerCharacter 0)))
    ;[0.15 0.15 0.15 0.5] Move towards player (Chase)
    (if (<= (Math|Vector|Distance(Vector) (Transformation|GetWorldLocation (Variables|Collision|GetCapsuleComponent)) (Transformation|GetWorldLocation (Variables|/Script/Engine.Character|GetCapsuleComponent _asbp_third_person_character))) (Variables|/Game/ThirdPerson/Blueprints/BP_ThirdPersonCharacter.BP_ThirdPersonCharacter_C|GetNoticableRange _asbp_third_person_character))
      (AI|AIMoveTo self "0, 0, 0" (Game|GetPlayerCharacter 0) 1e+02 false))))

(event Custom|Lunge%20at%20Player
  (if (not (Variables|Default|GetState))
    (bind _asbp_third_person_character (Utilities|Casting|CastToBP_ThirdPersonCharacter (Game|GetPlayerCharacter 0)))
    ;[0.15 0.15 0.15 0.5] Jump up and launch at player (Lunge)
    (if (<= (Math|Vector|Distance(Vector) (Transformation|GetWorldLocation (Variables|Collision|GetCapsuleComponent)) (Transformation|GetWorldLocation (Variables|/Script/Engine.Character|GetCapsuleComponent _asbp_third_person_character))) (Variables|/Game/ThirdPerson/Blueprints/BP_ThirdPersonCharacter.BP_ThirdPersonCharacter_C|GetNoticableRange _asbp_third_person_character))
      (Character|Jump)
      (Utilities|FlowControl|Delay 0.2)
      (Character|LaunchCharacter (* (Transformation|GetActorForwardVector self) 2e+03) false false))))

(event EventBeginPlay
  (bind _aswbp_rage_meter (Utilities|Casting|CastToWBP_RageMeter (UserInterface|GetWidget (Variables|Default|GetRageWidget))))
  ;[0.15 0.15 0.15 0.5] Move towards player (Chase)
  (Variables|/Game/Blueprints/WBP_RageMeter.WBP_RageMeter_C|SetMonkeyReference _aswbp_rage_meter self)
  (Utilities|Time|SetTimerbyEvent (delegate Custom|Chase%20Player) 0.2 true)
  ;[0.15 0.15 0.15 0.5] Jump up and launch at player (Lunge)
  (Utilities|Time|SetTimerbyEvent (delegate Custom|Lunge%20at%20Player) 4.0 true))

(event EventTick
  (params (DeltaSeconds :type Float%20%28single-precision%29))
  ;[0.15 0.15 0.15 0.5] upon defeat, stop moving and change player's condition
  (if (Variables|Default|GetState)
    (Components|Movement|StopMovementImmediately (Variables|Character|GetCharacterMovement))
    (bind _asbp_third_person_character (Utilities|Casting|CastToBP_ThirdPersonCharacter (Game|GetPlayerCharacter 0)))
    (Variables|/Game/ThirdPerson/Blueprints/BP_ThirdPersonCharacter.BP_ThirdPersonCharacter_C|SetBDefeat _asbp_third_person_character true)))

(fn ConstructionScript)