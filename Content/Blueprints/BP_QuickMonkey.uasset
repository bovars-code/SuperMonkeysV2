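; BP_QuickMonkey is an enemy character that chases and strafes around the player, dealing contact damage on capsule overlap and triggering fainting at zero health.
; Looping timers drive AI MoveTo and a left-right-right-left jump-dash sequence within the player's noticeable range, with launches based on player facing.
; BeginPlay links the monkey to its rage meter widget.
; While State is set, Tick halts movement and repeatedly calls the player's QuickDefeat.
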(event OnComponentBeginOverlap(CapsuleComponent)
  (params (OverlappedComponent :type Primitive%20Component%20Object%20Reference) (OtherActor :type Actor%20Object%20Reference) (OtherComp :type Primitive%20Component%20Object%20Reference) (OtherBodyIndex :type Integer) (bFromSweep :type Boolean) (SweepResult :type Hit%20Result%20Structure%20%28by%20ref%29))
  ;[0.15 0.15 0.15 0.5] Remove 5.0 from player's hp, check for faint scenario (Damage)
  (bind _asbp_third_person_character (Utilities|Casting|CastToBP_ThirdPersonCharacter OtherActor))
  (bind _output_get (Variables|/Game/ThirdPerson/Blueprints/BP_ThirdPersonCharacter.BP_ThirdPersonCharacter_C|SetHealth _asbp_third_person_character (- (Variables|/Game/ThirdPerson/Blueprints/BP_ThirdPersonCharacter.BP_ThirdPersonCharacter_C|GetHealth _asbp_third_person_character) 5.0)))
  (Development|PrintString (Utilities|String|ToString(Float) _output_get))
  (if (<= _output_get 0.0)
    (Default|Fainted _asbp_third_person_character)))

(event Custom|Chase%20Player
  (if (not (Variables|Default|GetState))
    (bind _asbp_third_person_character (Utilities|Casting|CastToBP_ThirdPersonCharacter (Game|GetPlayerCharacter 0)))
    (if (<= (Math|Vector|Distance(Vector) (Transformation|GetWorldLocation (Variables|Collision|GetCapsuleComponent)) (Transformation|GetWorldLocation (Variables|/Script/Engine.Character|GetCapsuleComponent _asbp_third_person_character))) (Variables|/Game/ThirdPerson/Blueprints/BP_ThirdPersonCharacter.BP_ThirdPersonCharacter_C|GetNoticableRange _asbp_third_person_character))
      ;[0.15 0.15 0.15 0.5] Move towards player (Chase)
      (AI|AIMoveTo self "0, 0, 0" (Game|GetPlayerCharacter 0) 1e+02 false))))

(event Custom|Strafe
  (if (not (Variables|Default|GetState))
    (bind _asbp_third_person_character (Utilities|Casting|CastToBP_ThirdPersonCharacter (Game|GetPlayerCharacter 0)))
    (if (<= (Math|Vector|Distance(Vector) (Transformation|GetWorldLocation (Variables|Collision|GetCapsuleComponent)) (Transformation|GetWorldLocation (Variables|/Script/Engine.Character|GetCapsuleComponent _asbp_third_person_character))) (Variables|/Game/ThirdPerson/Blueprints/BP_ThirdPersonCharacter.BP_ThirdPersonCharacter_C|GetNoticableRange _asbp_third_person_character))
      ;[0.15 0.15 0.15 0.5] Jumping around player (Strafe LRRL)
      (Character|Jump)
      (Utilities|FlowControl|Delay 0.1)
      (CallFunction|Dash true)
      (Utilities|FlowControl|Delay 0.5)
      (Character|Jump)
      (Utilities|FlowControl|Delay 0.1)
      (CallFunction|Dash false)
      (Utilities|FlowControl|Delay 0.5)
      (Character|Jump)
      (Utilities|FlowControl|Delay 0.1)
      (CallFunction|Dash false)
      (Utilities|FlowControl|Delay 0.5)
      (Character|Jump)
      (Utilities|FlowControl|Delay 0.1)
      (CallFunction|Dash true)
      (Utilities|FlowControl|Delay 0.5))))

(event EventBeginPlay
  (bind _aswbp_rage_meter (Utilities|Casting|CastToWBP_RageMeter (UserInterface|GetWidget (Variables|Default|GetRageWidget))))
  (Variables|/Game/Blueprints/WBP_RageMeter.WBP_RageMeter_C|SetMonkeyReference _aswbp_rage_meter self)
  ;[0.15 0.15 0.15 0.5] Move towards player (Chase)
  (Utilities|Time|SetTimerbyEvent (delegate Custom|Chase%20Player) 0.2 true)
  ;[0.15 0.15 0.15 0.5] Jumping around player (Strafe LRRL)
  (Utilities|Time|SetTimerbyEvent (delegate Custom|Strafe) 3.0 true))

(event EventTick
  (params (DeltaSeconds :type Float%20%28single-precision%29))
  (if (Variables|Default|GetState)
    (Components|Movement|StopMovementImmediately (Variables|Character|GetCharacterMovement))
    (bind _asbp_third_person_character (Utilities|Casting|CastToBP_ThirdPersonCharacter (Game|GetPlayerCharacter 0)))
    (Variables|/Game/ThirdPerson/Blueprints/BP_ThirdPersonCharacter.BP_ThirdPersonCharacter_C|SetQDefeat _asbp_third_person_character true)
    (Default|QuickDefeat _asbp_third_person_character)))

(fn ConstructionScript)

(fn Dash
  (params (Side :type Boolean))
  (bind _returnvalue (Game|GetPlayerCharacter 0))
  (bind _returnvalue_2 (Game|GetPlayerCharacter 0))
  (bind _returnvalue_3 (Transformation|GetActorRightVector _returnvalue))
  (bind _returnvalue_4 (Transformation|GetActorRightVector _returnvalue_2))
  (bind _returnvalue_5 (Math|Vector|NegateVector _returnvalue_4))
  (if Side
    (Character|LaunchCharacter (* (Math|Vector|Normalize (Math|Vector|NegateVector (+ (Transformation|GetActorForwardVector _returnvalue) _returnvalue_3 _returnvalue_3))) 1e+03) false false)
    (else
      (Character|LaunchCharacter (* (Math|Vector|Normalize (Math|Vector|NegateVector (+ (Transformation|GetActorForwardVector _returnvalue_2) _returnvalue_5 _returnvalue_5))) 1e+03) false false))))