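; BP_SneakyMonkey is an enemy character that chases the player with AI MoveTo and damages them on capsule hit, triggering a faint at zero health.
; While its State flag is false, a timer periodically flickers its light out, relocates it randomly among four hardcoded spots, then flickers back.
; When State is true, Tick stops movement, triggers the player's SneakDefeat, and updates a camera-facing rage meter widget from Health.
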(event OnComponentHit(CapsuleComponent)
  (params (HitComponent :type Primitive%20Component%20Object%20Reference) (OtherActor :type Actor%20Object%20Reference) (OtherComp :type Primitive%20Component%20Object%20Reference) (NormalImpulse :type Vector :default "0, 0, 0") (Hit :type Hit%20Result%20Structure%20%28by%20ref%29))
  ;[0.15 0.15 0.15 0.5] Remove 10.0 from player's hp, check for faint scenario (Damage)
  (bind _asbp_third_person_character (Utilities|Casting|CastToBP_ThirdPersonCharacter OtherActor))
  (bind _output_get (Variables|/Game/ThirdPerson/Blueprints/BP_ThirdPersonCharacter.BP_ThirdPersonCharacter_C|SetHealth _asbp_third_person_character (- (Variables|/Game/ThirdPerson/Blueprints/BP_ThirdPersonCharacter.BP_ThirdPersonCharacter_C|GetHealth _asbp_third_person_character) 5.0)))
  (Development|PrintString (Utilities|String|ToString(Float) _output_get))
  (if (<= _output_get 0.0)
    (Default|Fainted _asbp_third_person_character "Sneaky Monkey")))

(event Custom|Chase%20Player
  (if (not (Variables|Default|GetState))
    (AI|AIMoveTo self "0, 0, 0" (Game|GetPlayerCharacter 0) 1e+02 false)))

(event Custom|Hide
  (if (not (Variables|Default|GetState))
    (bind _alpha_track (Timeline|Off%20Flicker PlayFromStart)
      (:Update
        (Rendering|Components|Light|SetIntensity (Variables|/Script/Engine.Light|GetLightComponent (Variables|Default|GetLight)) (* _alpha_track 8.0)))
      (:Finished
        (Utilities|FlowControl|MultiGate true true -1
          (:Out%200
            (Transformation|SetActorLocation (Utilities|Array|Get(acopy) (Variables|Default|GetSneak_Coordinates)) true false)
            (bind _alpha_track_2 (Timeline|On%20Flicker PlayFromStart)
              (:Update
                (Rendering|Components|Light|SetIntensity (Variables|/Script/Engine.Light|GetLightComponent (Variables|Default|GetLight)) (* _alpha_track_2 8.0)))))
          (:Out%201
            (Transformation|SetActorLocation (Utilities|Array|Get(acopy) (Variables|Default|GetSneak_Coordinates) 1) true false)
            (Timeline|On%20Flicker PlayFromStart))
          (:Out%202
            (Transformation|SetActorLocation (Utilities|Array|Get(acopy) (Variables|Default|GetSneak_Coordinates) 2) true false)
            (Timeline|On%20Flicker PlayFromStart))
          (:Out%203
            (Transformation|SetActorLocation (Utilities|Array|Get(acopy) (Variables|Default|GetSneak_Coordinates) 3) true false)
            (Timeline|On%20Flicker PlayFromStart)))))))

(event EventTick
  (params (DeltaSeconds :type Float%20%28single-precision%29))
  (bind _ragewidget (Variables|Default|GetRageWidget))
  (if (Variables|Default|GetState)
    (Components|Movement|StopMovementImmediately (Variables|Character|GetCharacterMovement))
    (bind _asbp_third_person_character (Utilities|Casting|CastToBP_ThirdPersonCharacter (Game|GetPlayerCharacter 0)))
    (Variables|/Game/ThirdPerson/Blueprints/BP_ThirdPersonCharacter.BP_ThirdPersonCharacter_C|SetSDefeat _asbp_third_person_character true)
    (Default|SneakDefeat _asbp_third_person_character)
    ;[0.15 0.15 0.15 0.5] RageMeter
    (bind _aswbp_rage_meter (Utilities|Casting|CastToWBP_RageMeter (UserInterface|GetWidget (Variables|Default|GetRageWidget))))
    (Progress|SetPercent (Variables|/Game/Blueprints/WBP_RageMeter.WBP_RageMeter_C|GetRageMeter _aswbp_rage_meter) (/ (Variables|Default|GetHealth) 1e+02))
    (Transformation|SetWorldRotation _ragewidget (Math|Rotator|FindLookatRotation (Transformation|GetWorldLocation _ragewidget) (Transformation|GetWorldLocation (Variables|/Script/Engine.PlayerCameraManager|GetTransformComponent (Game|GetPlayerCameraManager 0)))) false false)))

(event Collision|EventActorBeginOverlap
  (params (OtherActor :type Actor%20Object%20Reference)))

(event EventBeginPlay
  (bind _aswbp_rage_meter (Utilities|Casting|CastToWBP_RageMeter (UserInterface|GetWidget (Variables|Default|GetRageWidget))))
  (Variables|/Game/Blueprints/WBP_RageMeter.WBP_RageMeter_C|SetMonkeyReference _aswbp_rage_meter self)
  (Utilities|Time|SetTimerbyEvent (delegate Custom|Chase%20Player) 0.2 true)
  (Variables|Default|SetSneak_Coordinates (Utilities|Array|MakeArray "6110.000000,-3870.000000,998.000000" "5110.000000,-4020.000000,998.000000" "4910.000000,-4020.000000,1418.000000" "7580.000000,-4020.000000,1418.000000" "7790.000000,-4020.000000,1038.000000" "7250.000000,-2940.000000,1038.000000" "6630.000000,-2820.000000,1128.000000" "7810.000000,-2360.000000,998.000000"))
  (Utilities|Time|SetTimerbyEvent (delegate Custom|Hide) 5.0 true))

(fn ConstructionScript)