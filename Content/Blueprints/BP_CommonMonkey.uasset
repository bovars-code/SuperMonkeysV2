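; BP_CommonMonkey is an enemy monkey that chases the player and damages them on contact.
; A looping timer issues AI move orders while State is false and the player is within their NoticableRange.
; While State is true, Tick halts movement, shows Health on the rage meter widget and turns it toward the camera.
; Capsule overlap with the player subtracts health and triggers Fainted at zero or below.
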(event OnComponentBeginOverlap(CapsuleComponent)
  (params (OverlappedComponent :type Primitive%20Component%20Object%20Reference) (OtherActor :type Actor%20Object%20Reference) (OtherComp :type Primitive%20Component%20Object%20Reference) (OtherBodyIndex :type Integer) (bFromSweep :type Boolean) (SweepResult :type Hit%20Result%20Structure%20%28by%20ref%29))
  ;[0.15 0.15 0.15 0.5] Remove 5.0 from player's hp, check for faint scenario (Damage)
  (bind _asbp_third_person_character (Utilities|Casting|CastToBP_ThirdPersonCharacter OtherActor))
  (bind _output_get (Variables|/Game/ThirdPerson/Blueprints/BP_ThirdPersonCharacter.BP_ThirdPersonCharacter_C|SetHealth _asbp_third_person_character (- (Variables|/Game/ThirdPerson/Blueprints/BP_ThirdPersonCharacter.BP_ThirdPersonCharacter_C|GetHealth _asbp_third_person_character) 5.0)))
  (Development|PrintString (Utilities|String|ToString(Float) _output_get))
  (if (<= _output_get 0.0)
    (Default|Fainted _asbp_third_person_character)))

(event Custom|Chase%20Player
  (if (not (Variables|Default|GetState))
    (bind _asbp_third_person_character (Utilities|Casting|CastToBP_ThirdPersonCharacter (Game|GetPlayerCharacter 0)))
    (if (<= (Math|Vector|Distance(Vector) (Transformation|GetWorldLocation (Variables|Collision|GetCapsuleComponent)) (Transformation|GetWorldLocation (Variables|/Script/Engine.Character|GetCapsuleComponent _asbp_third_person_character))) (Variables|/Game/ThirdPerson/Blueprints/BP_ThirdPersonCharacter.BP_ThirdPersonCharacter_C|GetNoticableRange _asbp_third_person_character))
      ;[0.15 0.15 0.15 0.5] Move towards player (Chase)
      (AI|AIMoveTo self "0, 0, 0" (Game|GetPlayerCharacter 0) 1e+02 false))))

(event EventBeginPlay
  (bind _aswbp_rage_meter (Utilities|Casting|CastToWBP_RageMeter (UserInterface|GetWidget (Variables|Default|GetRageWidget))))
  (Variables|/Game/Blueprints/WBP_RageMeter.WBP_RageMeter_C|SetMonkeyReference _aswbp_rage_meter self)
  ;[0.15 0.15 0.15 0.5] Move towards player (Chase)
  (Utilities|Time|SetTimerbyEvent (delegate Custom|Chase%20Player) 0.2 true))

(event EventTick
  (params (DeltaSeconds :type Float%20%28single-precision%29))
  (bind _ragewidget (Variables|Default|GetRageWidget))
  (if (Variables|Default|GetState)
    (Components|Movement|StopMovementImmediately (Variables|Character|GetCharacterMovement))
    (Utilities|Casting|CastToBP_ThirdPersonCharacter (Game|GetPlayerCharacter 0))
    (bind _aswbp_rage_meter (Utilities|Casting|CastToWBP_RageMeter (UserInterface|GetWidget (Variables|Default|GetRageWidget))))
    (Progress|SetPercent (Variables|/Game/Blueprints/WBP_RageMeter.WBP_RageMeter_C|GetRageMeter _aswbp_rage_meter) (/ (Variables|Default|GetHealth) 1e+02))
    (Transformation|SetWorldRotation _ragewidget (Math|Rotator|FindLookatRotation (Transformation|GetWorldLocation _ragewidget) (Transformation|GetWorldLocation (Variables|/Script/Engine.PlayerCameraManager|GetTransformComponent (Game|GetPlayerCameraManager 0)))) false false)))

(fn ConstructionScript)